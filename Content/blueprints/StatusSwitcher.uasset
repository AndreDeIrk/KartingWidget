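; StatusSwitcher turns NDI metadata into per-index status updates for map pointer, pointer and player widgets.
; ParseMetadata splits the "json" element by backslash; each entry is semicolon-split and forwarded, its first field toggling pointers and names.
; ShowMap also gates map pointers, though both handled cases hide the map.
; The GetActorOfClass chain that assigns widget references is unconnected and never runs.
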(event `MetadataReceived`
  (params (Metadata :type String))
  (bind _playersbp (`self.PlayersBP`))
  (bind _pointerbp (`self.PointerBP`))
  (bind _mappointerbp (`self.MapPointerBP`))
  (bind _mapbp (`self.MapBP`))
  (`|ExecutionSequence`
    (:`then_0`
      (bind _md (`self.ParseMetadata` Metadata)
        (:`Out`
          (for (_array_element _array_index) _md
            (`|ExecutionSequence`
              (:`then_0`
                (bind _returnvalue (`KismetStringLibrary.ParseIntoArray` _array_element ";" false))
                (`/Game/blueprints/widgets/MapPointerWidgetBP.SetPointerStatus` _mappointerbp _array_index _returnvalue)
                (switch `int` (`self.ShowMap`)
                  (:`0`
                    (`/Game/blueprints/widgets/MapWidgetBP.EventHideMap` _mapbp)
                    (`/Game/blueprints/widgets/MapPointerWidgetBP.HidePointer` _mappointerbp _array_index :!label _label))
                  (:`1`
                    (`/Game/blueprints/widgets/MapWidgetBP.EventHideMap` _mapbp)
                    (bind _returnvalue_2 (`KismetStringLibrary.Conv_StringToInt` (`|GetArrayItem` _returnvalue)))
                    (switch `int` _returnvalue_2
                      (:`0`
                        (goto _label))
                      (:`1`
                        (`/Game/blueprints/widgets/MapPointerWidgetBP.ShowPointer` _mappointerbp _array_index))))))
              (:`then_1`
                (`/Game/blueprints/widgets/PointerWidgetBP.SetPointerStatus` _pointerbp _array_index _returnvalue)
                (switch `int` _returnvalue_2
                  (:`0`
                    (`/Game/blueprints/widgets/PointerWidgetBP.HidePointer` _pointerbp _array_index))
                  (:`1`
                    (`/Game/blueprints/widgets/PointerWidgetBP.ShowPointer` _pointerbp _array_index))))
              (:`then_2`
                (`/Game/blueprints/widgets/PlayersWidgetBP.SetPlayerStatus` _playersbp _array_index _returnvalue)
                (switch `int` _returnvalue_2
                  (:`0`
                    (`/Game/blueprints/widgets/PlayersWidgetBP.EventHideName` _playersbp _array_index))
                  (:`1`
                    (`/Game/blueprints/widgets/PlayersWidgetBP.EventShowName` _playersbp _array_index)))))))))))

(fn `UserConstructionScript`)